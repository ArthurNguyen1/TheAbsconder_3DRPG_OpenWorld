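; BP_WaterBodyLake is a lake water volume that switches the player character in and out of swimming.
; Actor begin and end overlap events check for the Player tag, cast to BP_ThirdPersonCharacter, then call StartSwimming or StopSwimming on it.
; Each transition also prints a debug string, and the construction script is empty.
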(event Collision|EventActorBeginOverlap
  (params (OtherActor :type Actor%20Object%20Reference))
  (if (Actor|ActorHasTag OtherActor "Player")
    (bind _asbp_third_person_character (Utilities|Casting|CastToBP_ThirdPersonCharacter OtherActor))
    (Default|StartSwimming _asbp_third_person_character)
    (Development|PrintString "Swimming")))

(event Collision|EventActorEndOverlap
  (params (OtherActor :type Actor%20Object%20Reference))
  (if (Actor|ActorHasTag OtherActor "Player")
    (bind _asbp_third_person_character (Utilities|Casting|CastToBP_ThirdPersonCharacter OtherActor))
    (Default|StopSwimming _asbp_third_person_character)
    (Development|PrintString "Stop Swimming")))

(fn ConstructionScript)