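; BPC_Quest is a quest component that drives the on-screen quest HUD.
; On BeginPlay it creates a WB_QuestHUD widget, stores the reference and adds it to the viewport.
; Separate events push the ActiveQuest data to that widget, one setting the quest name text and the other passing the objective data to FillObjectives.
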(event Custom|Set%20Active%20Quest%20Text
  (Rendering|Components|TextRender|SetText (Variables|/Game/Quest_System/WB_QuestHUD.WB_QuestHUD_C|GetActiveQuestText (Variables|Default|GetQuest%20HUD%20Widget)) (Utilities|Text|ToText(String) (.Name (Utilities|Struct|BreakS_Quest (Variables|Default|GetactiveQuest))))))

(event Custom|Set%20Objectives
  (Default|FillObjectives (Variables|Default|GetQuest%20HUD%20Widget) (.objective (Variables|Default|GetactiveQuest))))

(event EventBeginPlay
  (bind _returnvalue (UserInterface|CreateWidget "/Game/Quest_System/WB_QuestHUD.WB_QuestHUD_C"))
  (bind _output_get (Variables|Default|SetQuest%20HUD%20Widget _returnvalue))
  (UserInterface|Viewport|AddtoViewport _output_get 0))